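; Debug actor that simulates bullet drop from an arrow component and draws it beside Unreal's predicted projectile path.
; BulletDropCalc steps the trajectory in SimFrequency segments, adding gravity per step and drawing debug lines and spheres until a line trace hits.
; It then resets position and velocity.
; BeginPlay reruns this simulation and the built-in PredictProjectilePath every 1.5 seconds with shared start parameters.
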(event `Bullet Drop Calc`
  (bind _velocity (`self.Velocity`))
  (bind _end (`self.End`))
  (bind _max_sim_time (`self.Max Sim Time`))
  (set `self.End` (+ (`self.Start`) (/ (`self.Velocity`) (`KismetMathLibrary.MakeVector` (`self.Sim Frequency`) 1.0 1.0))))
  (for _ (range (+ (`KismetMathLibrary.FTrunc` (`self.Sim Frequency`)) 1))
    (`KismetSystemLibrary.DrawDebugLine` (`self.Start`) _end (struct :`R` 1.0 :`B` 0.275878 :`A` 1.0) _max_sim_time)
    (`KismetSystemLibrary.DrawDebugSphere` _end 5.0 12 (struct :`G` 0.765195 :`B` 1.0 :`A` 1.0) _max_sim_time)
    (bind (_outhit _returnvalue) (`KismetSystemLibrary.LineTraceSingleByProfile` (`self.Start`) (`self.End`) "BlockAll"))
    (if _returnvalue
      (break)
      (else
        (set `self.Start` (`self.End`))
        (set `self.Velocity` (+ _velocity (`KismetMathLibrary.MakeVector` 0.0 0.0 (/ -980.0 (`KismetMathLibrary.Square` (`self.Sim Frequency`))))))
        (set `self.End` (+ (`self.Start`) (/ _velocity (`KismetMathLibrary.MakeVector` (`self.Sim Frequency`) 1.0 1.0)))))))
  (set `self.Start` (`SceneComponent.K2_GetComponentLocation` (`self.Arrow`)))
  (set `self.Velocity` (`self.Starting Velocity`)))

(event `self.ReceiveBeginPlay`
  (bind _output_get (set `self.Start` (`SceneComponent.K2_GetComponentLocation` (`self.Arrow`))))
  (`|ExecutionSequence` :!label _label
    (:`then_0`
      (`self.Bullet Drop Calc`))
    (:`then_1`
      (`GameplayStatics.Blueprint_PredictProjectilePath_Advanced` (make `PredictProjectilePathParams` _output_get (`self.Starting Velocity`) true 0.0 (`self.Max Sim Time`) true "ECC_WorldStatic" _ _ (`self.Sim Frequency`) 0.0 "ForDuration"))
      (`KismetSystemLibrary.Delay` 1.5)
      (goto _label))))

(fn `UserConstructionScript`)