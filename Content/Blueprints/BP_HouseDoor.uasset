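; BP_HouseDoor is a house door actor with an OpenHouseDoor event meant to swing its mesh open.
; A Timeline lerps the mesh's relative rotation and, on every update, calls AddUnique on OpenedHouseDoor in the GM_Coding2ForReal game mode's LevelSave2.
; The Timeline sits behind a Branch fixed to false, so it never plays.
; Camera blends to the door and back are disconnected, leaving the NewViewTarget input unused.
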(event `OpenHouseDoor`
  (params (NewViewTarget :type "Actor Object Reference"))
  (if false
    (bind (_direction _newtrack_0) (`Timeline|Timeline`)
      (:`Update`
        (`SceneComponent.K2_SetRelativeRotation` (`self.SM_Bld_Door_01`) (`KismetMathLibrary.RLerp` (struct) (struct :`Yaw` 180.0) _newtrack_0) false false)
        (bind _asgm_coding_2for_real (cast `/Game/Blueprints/NewSaves/GM_Coding2ForReal` (`GameplayStatics.GetGameMode`)))
        (`KismetArrayLibrary.Array_AddUnique` (`/Game/Blueprints/NewSaves/SG_LevelSave2.OpenedHouseDoor` (`/Game/Blueprints/NewSaves/GM_Coding2ForReal.LevelSave2` _asgm_coding_2for_real)))))))

(fn `UserConstructionScript`)