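; BP_ItemPickup is a placeable item pickup that hovers in place until it is picked up.
; The construction script assigns the ItemModelToPlace mesh to the SMPoolNoodle component, letting one Blueprint show different items.
; On BeginPlay, the Float timeline drives that mesh's relative location to animate it.
; The PickUp event prints a debug message, waits a tick and destroys the actor.
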(event `self.ReceiveBeginPlay`
  (bind (_direction _z_axis) (`Timeline|Float`)
    (:`Update`
      (`SceneComponent.K2_SetRelativeLocation` (`self.SM_PoolNoodle`) _z_axis false false))))

(event `/Game/Blueprints/BPI_Item.PickUp`
  (`KismetSystemLibrary.PrintString` "Item Picked Up")
  (`KismetSystemLibrary.DelayUntilNextTick`)
  (`self.K2_DestroyActor`))

(fn `UserConstructionScript`
  (`StaticMeshComponent.SetStaticMesh` (`self.SM_PoolNoodle`) (`self.ItemModelToPlace`)))