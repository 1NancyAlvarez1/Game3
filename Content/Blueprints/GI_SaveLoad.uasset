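; Game instance blueprint sketching save, load and delete for player and level data, with its logic currently disconnected.
; Checkpoint only logs a message; the other events are empty.
; Unreachable chains copy stamina, transform and sprint/shoot flags between character and SG_Coding2, and use level names as level save slots.
; The player load chain crosses the sprint and shoot flags.
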(event `Checkpoint`
  (`KismetSystemLibrary.LogString` "Loading Checkpoint"))

(event `Save Player`
  ;[0.9563 1 0.3152 1 34] Save
)

(event `Load Player`
  ;[0.1494 1 0] Load
)

(event `Save Level`)

(event `Load Level`)

(event `Delete Save Data`)

(event `self.ReceiveInit`)