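; GM_Coding2ForReal is a game mode that manages per-level saves through an SG_LevelSave2 object, using the level name as slot name.
; On BeginPlay it creates that object or loads it, restoring doors, triggers, coins, sword and house state.
; The player's capsule moves to the saved transform unless its location is zero.
; Checkpoint stores a transform and saves, while FinishLevel clears it so the next load skips repositioning.
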(event `self.ReceiveBeginPlay`
  (bind _levelsave2 (`self.LevelSave2`))
  (bind _playertransform_location (`KismetMathLibrary.BreakTransform` (`/Game/Blueprints/NewSaves/SG_LevelSave2.PlayerTransform` _levelsave2)))
  (`KismetSystemLibrary.PrintString` "Loaded into the GM_Coding2ForReal" true true (struct :`R` 1.0 :`B` 0.03671 :`A` 1.0) 20.0)
  (bind _returnvalue (`GameplayStatics.GetCurrentLevelName` true))
  (bind _returnvalue_2 (`GameplayStatics.DoesSaveGameExist` _returnvalue))
  (if _returnvalue_2
    (bind _returnvalue_3 (`GameplayStatics.LoadGameFromSlot` _returnvalue))
    (bind _assg_level_save_2 (cast `/Game/Blueprints/NewSaves/SG_LevelSave2` _returnvalue_3))
    (bind _output_get (set `self.LevelSave2` _assg_level_save_2))
    (`|ExecutionSequence`
      (:`then_0`
        (`/Game/Blueprints/NewSaves/SG_LevelSave2.LoadSavedDoor` _output_get))
      (:`then_1`
        (`/Game/Blueprints/NewSaves/SG_LevelSave2.LoadCollectedCoins` _output_get)
        (if (not (`KismetMathLibrary.EqualExactly_VectorVector` _playertransform_location))
          (`SceneComponent.K2_SetWorldTransform` (`Character.CapsuleComponent` (`GameplayStatics.GetPlayerCharacter` 0)) (`/Game/Blueprints/NewSaves/SG_LevelSave2.PlayerTransform` _levelsave2) false false)))
      (:`then_2`
        (`/Game/Blueprints/NewSaves/SG_LevelSave2.LoadSavedTrigger` _output_get))
      (:`then_3`
        (`/Game/Blueprints/NewSaves/SG_LevelSave2.LoadCollectedSword` _output_get))
      (:`then_4`
        (`/Game/Blueprints/NewSaves/SG_LevelSave2.LoadHouseDoor` _output_get))
      (:`then_5`
        (`/Game/Blueprints/NewSaves/SG_LevelSave2.LoadHouseTrigger` _output_get)))
    (else
      (bind _returnvalue_4 (`GameplayStatics.CreateSaveGameObject` "/Game/Blueprints/NewSaves/SG_LevelSave2.SG_LevelSave2_C"))
      (set `self.LevelSave2` _returnvalue_4))))

(event `Save Game`
  (bind _returnvalue (`GameplayStatics.GetCurrentLevelName` true))
  (bind _returnvalue_2 (`GameplayStatics.SaveGameToSlot` (`self.LevelSave2`) _returnvalue))
  (if _returnvalue_2
    _))

(fn `Checkpoint`
  (params (`Player Transform` :type "Transform Structure"))
  (set `/Game/Blueprints/NewSaves/SG_LevelSave2.PlayerTransform` `Player Transform` (`self.LevelSave2`))
  (`self.Save Game`))

(fn `FinishLevel`
  (set `/Game/Blueprints/NewSaves/SG_LevelSave2.PlayerTransform` (struct) (`self.LevelSave2`)) ; Reset player start location to 0,0,0
  (`self.Save Game`))

(fn `UserConstructionScript`)