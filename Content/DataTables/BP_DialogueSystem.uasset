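; Dialogue actor that lets the player step through DT_TestDialogue with E while inside its sphere, after a brief key prompt on entry.
; Each press advances RowIndex, showing the row's text and emotion in W_DataTableDialogue and playing its voice sound.
; The speaker portrait comes from offsetting a dynamic material's UV Location per speaker.
; Past the last row the widget is removed and its show-once gate resets, but RowIndex is never rewound.
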(event `self.ReceiveBeginPlay`
  (bind _returnvalue (`|CreateWidget` "/Game/WidgetsUI/W_DataTableDialogue.W_DataTableDialogue_C"))
  (bind _output_get (set `self.W_Dialogue` _returnvalue)))

(event `debug system`)

(event `NextLine`
  (bind _row_index (`self.Row Index`))
  (`|ExecutionSequence`
    (:`then_0`
      (`/Engine/EditorBlueprintResources/StandardMacros.DoOnce` false :!label _label
        (:`Completed`
          (`UserWidget.AddToViewport` (`self.W_Dialogue`) 0))))
    (:`then_1`
      (bind _outrownames (`DataTableFunctionLibrary.GetDataTableRowNames` "/Game/DataTables/DT_TestDialogue.DT_TestDialogue"))
      (if (< _row_index (`KismetArrayLibrary.Array_Length` _outrownames))
        (bind _returnvalue (`|GetDataTableRow` "/Game/DataTables/DT_TestDialogue.DT_TestDialogue" (`|GetArrayItem` _outrownames _row_index))
          (:`then`
            (`TextBlock.SetText` (`/Game/WidgetsUI/W_DataTableDialogue.TextBlock_79` (stale `self.ReceiveBeginPlay` _output_get)) (break `/Game/DataTables/S_DialogueLine` _returnvalue))
            (`TextBlock.SetText` (`/Game/WidgetsUI/W_DataTableDialogue.TextBlock_0` (stale `self.ReceiveBeginPlay` _output_get)) (`KismetTextLibrary.Conv_StringToText` (`|GetEnumeratorNameAsString` (`.Emotion_11_4BD1DA30497EECC3355066A836942ED7` (break `/Game/DataTables/S_DialogueLine` _returnvalue)))))
            (`GameplayStatics.PlaySoundAtLocation` (`.SpokenText_10_20ABA97A4A97EF5C5E524F86481A12E2` (break `/Game/DataTables/S_DialogueLine` _returnvalue)) (0.0 0.0 0.0) (struct) 1.0 1.0 0.0 null null null null)
            (bind _image_190 (`/Game/WidgetsUI/W_DataTableDialogue.Image_190` (stale `self.ReceiveBeginPlay` _output_get)))
            (bind _returnvalue_2 (`Image.GetDynamicMaterial` _image_190))
            (`Image.SetBrushFromMaterial` _image_190 _returnvalue_2)
            (bind (_returnvalue_x _returnvalue_y) (`KismetMathLibrary.BreakVector` (select `/Game/DataTables/E_Character` (`.Speaker_12_3C529EE3445801EDACB64E83CC33CDCC` (break `/Game/DataTables/S_DialogueLine` _returnvalue)) :`NewEnumerator0` (1.2 1.2 0.0) :`NewEnumerator1` (2.3 1.2 0.0) :`NewEnumerator3` (1.2 0.0 0.0) :`NewEnumerator4` (0.0 2.2 0.0) :`NewEnumerator5` (1.2 2.3 0.0) :`NewEnumerator6` (2.3 0.0 0.0) :`NewEnumerator7` (2.3 2.3 0.0) :`NewEnumerator8` (0.0 1.2 0.0) :!type "Vector Structure")))
            (`MaterialInstanceDynamic.SetVectorParameterValue` _returnvalue_2 "UV Location" (make `LinearColor` _returnvalue_x _returnvalue_y 0.0 1.0))
            (`/Engine/EditorBlueprintResources/StandardMacros.IncrementInt` (`self.Row Index`))))
        (else
          (`Widget.RemoveFromParent` (`self.W_Dialogue`))
          (`self.reset add to view`))))))

(event `reset add to view`
  (goto _label :!via `Reset`))

(event `self.Sphere.OnComponentBeginOverlap`
  (params (OverlappedComponent :type "PrimitiveComponent Object Reference") (OtherActor :type "Actor Object Reference") (OtherComp :type "PrimitiveComponent Object Reference") (OtherBodyIndex :type Integer) (bFromSweep :type Boolean) (SweepResult :type "HitResult Structure (by ref)"))
  (cast `/Game/ThirdPerson/Blueprints/BP_ThirdPersonCharacter` OtherActor)
  (`self.EnableInput` (`GameplayStatics.GetPlayerController` 0))
  (bind _returnvalue (`|CreateWidget` "/Game/WidgetsUI/W_PressE.W_PressE_C"))
  (`UserWidget.AddToViewport` _returnvalue 0)
  (`KismetSystemLibrary.Delay` 2.0)
  (`Widget.RemoveFromParent` _returnvalue))

(event `self.Sphere.OnComponentEndOverlap`
  (params (OverlappedComponent :type "PrimitiveComponent Object Reference") (OtherActor :type "Actor Object Reference") (OtherComp :type "PrimitiveComponent Object Reference") (OtherBodyIndex :type Integer))
  (cast `/Game/ThirdPerson/Blueprints/BP_ThirdPersonCharacter` OtherActor)
  (`self.DisableInput` (`GameplayStatics.GetPlayerController` 0)))

(event `Key|E`
  (params (Key :type "Key Structure"))
  (:`Pressed`
    (`self.NextLine`)))

(fn `UserConstructionScript`)