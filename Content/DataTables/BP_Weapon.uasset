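; BP_Weapon is a weapon actor with a mesh and text labels for its weapon type, elemental type and damage range.
; RandomizeValues nudges the minimum damage by a small random amount, derives the maximum from it, then refreshes the labels and applies the WeaponMesh variable to WeaponBody.
; AddTexture is an empty stub, and a mesh lookup by weapon type is left unconnected.
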(event `SetMesh`
  (`StaticMeshComponent.SetStaticMesh` (`self.WeaponBody`) (`self.WeaponMesh`)))

(event `Randomize Values`
  (bind _output_get (set `self.MinDmg` (+ (`self.MinDmg`) (`KismetMathLibrary.RandomInteger` 2))))
  (set `self.MaxDmg` (+ _output_get (`KismetMathLibrary.RandomIntegerInRange` 1 4)))
  (`self.UpdateText`)
  (`self.SetMesh`))

(event `UpdateText`
  (`TextRenderComponent.K2_SetText` (`self.TextWeaponType`) (`KismetTextLibrary.Conv_StringToText` (`|GetEnumeratorNameAsString` (`self.WeaponType`))))
  (`TextRenderComponent.K2_SetText` (`self.TextElementalType`) (`KismetTextLibrary.Conv_StringToText` (`|GetEnumeratorNameAsString` (`self.ElementalType`))))
  (`TextRenderComponent.K2_SetText` (`self.TextDmg`) (`KismetTextLibrary.Conv_StringToText` (`KismetStringLibrary.Concat_StrStr` (`KismetStringLibrary.Conv_IntToString` (`self.MinDmg`)) "-" (`KismetStringLibrary.Conv_IntToString` (`self.MaxDmg`))))))

(event `AddTexture`)

(event `self.ReceiveBeginPlay`)

(fn `UserConstructionScript`)