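; Binoculars skill pickup that attaches to the player's face socket on overlap and zooms the first-person camera while held.
; Holding drives an FOV timeline and shows the ring widget on the first enemy found.
; Self-calling delay loops drain duration and mana, then run a cooldown equal to time used.
; A separate Z-key branch switches the camera's post-process material and the enemy ring.
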(event `self.HoldSkill`
  ;[1 1 1] Comment
  (if (`self.Skill Is Active`)
    (bind _result (`/Engine/EditorBlueprintResources/StandardMacros.IncrementInt` (`self.Hold Count`))
      (:`  `
        (`KismetSystemLibrary.PrintString` (`KismetStringLibrary.Concat_StrStr` "This skill has been held down for " (`KismetStringLibrary.Conv_IntToString` _result) " frames.") true true (struct :`R` 1.0 :`G` 0.541323 :`A` 1.0) 0.0)
        (`self.ActivateRing`)
        (`self.Zoom`)))))

(event `Zoom`
  ;[1 1 1] Zoom
  (bind _asbp_third_person_character (cast `/Game/ThirdPerson/Blueprints/BP_ThirdPersonCharacter` (`GameplayStatics.GetPlayerPawn` 0)))
  (set `self.IsZoom?` true)
  (bind (_direction _fov) (`Timeline|T_Zoom` :!label _label)
    (:`Update`
      (`CameraComponent.SetFieldOfView` (`/Game/ThirdPerson/Blueprints/BP_ThirdPersonCharacter.FirstPersonCamera` _asbp_third_person_character) _fov)
      (`KismetSystemLibrary.Delay` 6.0)
      (`KismetSystemLibrary.PrintString` "Zoom in"))))

(event `self.EndSkill`
  ;[1 1 1] Stop early
  (`self.Stop Zoom`)
  (`self.DeactivateRing`)
  ;[1 1 1] Zoom
  (set `self.IsZoom?` false :!label _label_2)
  (goto _label :!via `Reverse`))

(event `Stop Zoom`
  ;[1 1 1] Stop Zooming
  (if (`self.Skill is Active`)
    (set `self.Skill is Active` false)
    (set `self.Skill Cooldown` (- 5.0 (`self.Skill Duration`))) ; subtract whatever time the \nplayer still had for this effect
    (set `self.Skill Duration` 5.0) ; reset skill duration
    (set `self.Hold Count` 0)
    (`GameplayStatics.PlaySoundAtLocation` "/Game/TeamLuigi/Nancy/RZoomSFX.RZoomSFX" (`SceneComponent.K2_GetComponentLocation` (`self.DefaultSceneRoot`)) (struct) 1.0 1.0 0.0 null null null null)
    (`self.Update Cooldown`)
    (`self.DeactivateRing`)
    (goto _label_2)
    (else
      (`KismetSystemLibrary.PrintString` "skill is already inactive"))))

(event `Key|Z`
  (params (Key :type "Key Structure"))
  (:`Pressed`
    (cast `/Game/ThirdPerson/Blueprints/BP_ThirdPersonCharacter` (`GameplayStatics.GetPlayerPawn` 0))
    (set `self.KeyInput` "Z")
    (if (`self.IsZ?`)
      (`self.ActivateRing`)
      (set `self.PostProcessEnable` true)
      (`self.Post Process Set Up` "/Game/TeamLuigi/Nancy/M_PostProcess_Inst.M_PostProcess_Inst")
      (`Timeline|Timeline_2` :!label _label_3
        (:`Finished`
          (if (not (`self.PostProcessEnable`))
            (`self.Post Process Set Up` "/Game/TeamLuigi/Nancy/M_PostProcess.M_PostProcess"))))
      (else
        (`self.DeactivateRing`)
        (set `self.PostProcessEnable` false)
        (goto _label_3 :!via `Reverse`)))))

(event `self.BeginSkill`
  ;[1 1 1] Begin Skill
  (`KismetSystemLibrary.PrintString` "Begin BF Skill")
  (if (<= (`self.Skill Cooldown`) 0.0)
    (set `self.Skill is Active` true)
    (`GameplayStatics.PlaySoundAtLocation` "/Game/TeamLuigi/Nancy/Zoom1SFX.Zoom1SFX" (`SceneComponent.K2_GetComponentLocation` (`self.DefaultSceneRoot`)) (struct) 1.0 1.0 0.0 null null null null)
    (`self.Update Time Remaining`)
    (else
      (`self.Stop Zoom`))))

(event `Update Time Remaining`
  (bind _skill_duration (`self.Skill Duration`))
  ;[1 1 1] Time Remaining
  (if (`self.Skill is Active`)
    (set `self.Skill Duration` (- _skill_duration 0.1))
    (if (>= _skill_duration 0.0)
      (bind (_isalive _hasmana) (`/Game/ThirdPerson/Blueprints/BP_ThirdPersonCharacter.Update Player Stats` (`self.As BP Third Person Character`) 0.0 -0.02 0.0))
      (if _hasmana
        (`KismetSystemLibrary.Delay` 0.1)
        (`self.Update Time Remaining`)
        (else
          (`self.Stop Zoom` :!label _label_4)
          (`KismetSystemLibrary.PrintString` "No mana left")))
      (else
        (goto _label_4)))))

(event `ActivateRing`
  ;[1 0.3125 0.3125] Activate
  (bind _outactors (`GameplayStatics.GetAllActorsOfClass` "/Game/TeamLuigi/Nancy/BP_EditedEnemy_Base.BP_EditedEnemy_Base_C"))
  (`/Game/TeamLuigi/Nancy/W_Ring.ShowRing` (`/Game/TeamLuigi/Nancy/BP_EditedEnemy_Base.As Ring Widget` (`|GetArrayItem` _outactors))))

(event `Update Cooldown`
  ;[1 1 1] Cooldown
  (if (> (`self.Skill Cooldown`) 0.0)
    (bind _output_get (set `self.Skill Cooldown` (- (`self.Skill Cooldown`) 0.1)))
    (`KismetSystemLibrary.Delay` 0.1)
    (`KismetSystemLibrary.PrintString` (`KismetStringLibrary.Concat_StrStr` "Binocular cooldown is" (`KismetStringLibrary.Conv_DoubleToString` _output_get)) true true (struct :`G` 0.66 :`B` 1.0 :`A` 1.0) 0.1)
    (`self.Update Cooldown`)))

(event `DeactivateRing`
  ;[0.1406 0.06958 0.06958] Deactivate
  (bind _outactors (`GameplayStatics.GetAllActorsOfClass` "/Game/TeamLuigi/Nancy/BP_EditedEnemy_Base.BP_EditedEnemy_Base_C"))
  (`/Game/TeamLuigi/Nancy/W_Ring.HideRing` (`/Game/TeamLuigi/Nancy/BP_EditedEnemy_Base.As Ring Widget` (`|GetArrayItem` _outactors))))

(event `self.Collision.OnComponentBeginOverlap`
  (params (OverlappedComponent :type "PrimitiveComponent Object Reference") (OtherActor :type "Actor Object Reference") (OtherComp :type "PrimitiveComponent Object Reference") (OtherBodyIndex :type Integer) (bFromSweep :type Boolean) (SweepResult :type "HitResult Structure (by ref)"))
  ;[1 1 1] Grab skill once
  (bind _asbp_third_person_character (cast `/Game/ThirdPerson/Blueprints/BP_ThirdPersonCharacter` OtherActor))
  (bind _output_get (set `self.As BP Third Person Character` _asbp_third_person_character)) ; We'll need this for mana, ammo, and other checks
  (`/Game/ThirdPerson/Blueprints/BP_ThirdPersonCharacter.CurrentSKill` _output_get
    (:`then`
      (`KismetSystemLibrary.PrintString` "You're already holding a skill!"))
    (:`else`
      (set `self.Current SKill` self)
      (`self.K2_AttachToComponent` (`Character.Mesh` _output_get) "face" "SnapToTarget" "SnapToTarget" "SnapToTarget") ; attach this skill to the player's left hand
    )))

(fn `Post Process Set Up`
  (params (Object :type "Object Object Reference"))
  (bind _asbp_third_person_character (cast `/Game/ThirdPerson/Blueprints/BP_ThirdPersonCharacter` (`GameplayStatics.GetPlayerPawn` 0)))
  (set `CameraComponent.PostProcessSettings` (make `PostProcessSettings` :`WeightedBlendables` (make `WeightedBlendables` (`|MakeArray` (make `WeightedBlendable` 1.0 Object)))) (`/Game/ThirdPerson/Blueprints/BP_ThirdPersonCharacter.FirstPersonCamera` _asbp_third_person_character)))

(fn `Stop Skill`)

(fn `Update Skill Cooldown`)

(fn `Update Skill Duration`)

(fn `UserConstructionScript`)